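; BP_HTTP_Template_Oatpp is a template Blueprint that launches an Oat++ HTTP server from the FF_HTTP_OATPP plugin at BeginPlay.
; It builds absolute paths to the web root and 404 page inside the plugin's Resources/wwwroot folder.
; A custom event then spawns the HTTP_Server_Oatpp actor with those paths and a server name, and stores a reference to it.
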(event `self.ReceiveBeginPlay`
  (bind _outbasedir (`PluginBlueprintLibrary.GetPluginBaseDir` "FF_HTTP_OATPP"))
  (set `self.Path_Root` (`KismetSystemLibrary.ConvertToAbsolutePath` (`KismetStringLibrary.Concat_StrStr` _outbasedir "/Resources/wwwroot/root")))
  (set `self.Path_404` (`KismetSystemLibrary.ConvertToAbsolutePath` (`KismetStringLibrary.Concat_StrStr` _outbasedir "/Resources/wwwroot/404.html")))
  (`self.Event_Oatpp`))

(event `Event_Oatpp`
  (bind _returnvalue (`|SpawnActorFromClass` "/Script/FF_HTTP_OATPP.HTTP_Server_Oatpp" (`KismetMathLibrary.MakeTransform` (0.0 0.0 0.0)) "Undefined" "MultiplyWithRoot" null (`self.Path_Root`) (`self.Path_404`) "http://0.0.0.0:8081" "api/*" "oatpp" null))
  (set `self.REF_Oatpp` _returnvalue))

(fn `UserConstructionScript`)