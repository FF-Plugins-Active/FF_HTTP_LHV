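; Template actor that runs an embedded HTTP server from the FF_HTTP_LHV plugin as a usage example.
; On BeginPlay it resolves the plugin's web root and 404 page paths, spawns a multithreaded server actor and binds start, stop and request delegates that print status.
; Each request prints its headers and gets a random plain-text name in reply.
; Disconnected nodes hold fuller request inspection and an alternative send call.
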(event `Delegate_HTTP_LibHv_Start`
  (`KismetSystemLibrary.PrintString` "HTTP Started" true true (struct :`G` 1.0 :`A` 1.0) 20.0))

(event `self.ReceiveBeginPlay`
  (bind (_outbasedir _returnvalue) (`PluginBlueprintLibrary.GetPluginBaseDir` "FF_HTTP_LHV"))
  (if _returnvalue
    (set `self.Path_Root` (`KismetSystemLibrary.ConvertToAbsolutePath` (`KismetStringLibrary.Concat_StrStr` _outbasedir "/Resources/wwwroot/root/")))
    (set `self.Path_404` (`KismetSystemLibrary.ConvertToAbsolutePath` (`KismetStringLibrary.Concat_StrStr` _outbasedir "/Resources/wwwroot/404.html"))))
  (bind _returnvalue_2 (`|SpawnActorFromClass` "/Script/FF_HTTP_LHV.HTTP_Server_LHV" (`KismetMathLibrary.MakeTransform` (0.0 0.0 0.0)) "Undefined" "MultiplyWithRoot" null (`self.Path_Root`) (`self.Path_404`) 8081 8453 4 "/api/libhv/v1" "HTTP_Server_LibHv" null))
  (set `self.Server_LHV` _returnvalue_2)
  (`|ExecutionSequence`
    (:`then_0`
      (add `HTTP_Server_LHV.Delegate_HTTP_LibHv_Start` (`self.Server_LHV`) (delegate `Delegate_HTTP_LibHv_Start`)))
    (:`then_1`
      (add `HTTP_Server_LHV.Delegate_HTTP_LibHv_Stop` (`self.Server_LHV`) (delegate `Delegate_HTTP_LibHv_Stop`)))
    (:`then_2`
      (add `HTTP_Server_LHV.Delegate_HTTP_LibHv_Request` (`self.Server_LHV`) (delegate `Delegate_HTTP_LibHv_Request`)))))

(event `Delegate_HTTP_LibHv_Stop`
  (`KismetSystemLibrary.PrintString` "HTTP Stopped" true true (struct :`R` 1.0 :`A` 1.0) 20.0))

(event `Delegate_HTTP_LibHv_Request`
  (params (Connection :type "HttpConnectionLhv Object Reference"))
  (`self.F_Give_Response_LibHv` Connection))

(fn `F_Give_Response_LibHv`
  (params (Connection :type "HttpConnectionLhv Object Reference"))
  (locals (LOC_Connection :type "HttpConnectionLhv Object Reference") (LOC_Querries :type String) (LOC_Client_Addr :type String) (LOC_Paths :type String) (LOC_Body :type String) (LOC_Contenty_Type :type String) (LOC_All_Headers :type String) (LOC_Single_Header :type String))
  (set `local.LOC_Connection` Connection)
  (`KismetSystemLibrary.PrintString` (`.Out_String` (`HttpConnectionLhv.GetHeaders` (`local.LOC_Connection`))) true true (struct :`G` 0.66 :`B` 1.0 :`A` 1.0) 10.0)
  (bind _returnvalue (`HttpConnectionLhv.SendResponse` (`local.LOC_Connection`) (`KismetArrayLibrary.Array_Random` (`|MakeArray` "Eray" "Ezgi" "Burak")) (`|MakeMap` "Content-Type" "text/plain") "OK_200" "Text_Plain"))
  (return))

(fn `UserConstructionScript`)