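; Template actor that runs a LibHv-based HTTP server from the FF_HTTP_LHV plugin and answers incoming requests.
; On BeginPlay it resolves the plugin's wwwroot and 404 paths, copies the root path to the clipboard, spawns the server actor and binds start, stop and request delegates.
; Each request's details are gathered and printed on screen, and a random name is sent back as plain text.
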(event `Delegate_HTTP_LibHv_Start`
  (`KismetSystemLibrary.PrintString` "HTTP Started" true true (struct :`G` 1.0 :`A` 1.0) 20.0))

(event `self.ReceiveBeginPlay`
  (bind (_outbasedir _returnvalue) (`PluginBlueprintLibrary.GetPluginBaseDir` "FF_HTTP_LHV"))
  (if _returnvalue
    (bind _output_get (set `self.Path_Root` (`KismetSystemLibrary.ConvertToAbsolutePath` (`KismetStringLibrary.Concat_StrStr` _outbasedir "/Resources/wwwroot/root/"))))
    (`LowEntryExtendedStandardLibrary.ClipboardSet` _output_get)
    (set `self.Path_404` (`KismetSystemLibrary.ConvertToAbsolutePath` (`KismetStringLibrary.Concat_StrStr` _outbasedir "/Resources/wwwroot/404.html"))))
  (bind _returnvalue_2 (`|SpawnActorFromClass` "/Script/FF_HTTP_LHV.HTTP_Server_LHV" (`KismetMathLibrary.MakeTransform` (0.0 0.0 0.0)) "Undefined" "MultiplyWithRoot" null (`self.Path_Root`) (`self.Path_404`) 8081 8453 4 "/api/libhv/v1/" "LibHv" null))
  (set `self.Server_LHV` _returnvalue_2)
  (`|ExecutionSequence`
    (:`then_0`
      (add `HTTP_Server_LHV.Delegate_HTTP_LibHv_Start` (`self.Server_LHV`) (delegate `Delegate_HTTP_LibHv_Start`)))
    (:`then_1`
      (add `HTTP_Server_LHV.Delegate_HTTP_LibHv_Stop` (`self.Server_LHV`) (delegate `Delegate_HTTP_LibHv_Stop`)))
    (:`then_2`
      (add `HTTP_Server_LHV.Delegate_HTTP_LibHv_Request` (`self.Server_LHV`) (delegate `Delegate_HTTP_LibHv_Request`)))))

(event `Delegate_HTTP_LibHv_Stop`
  (`KismetSystemLibrary.PrintString` "HTTP Stopped" true true (struct :`R` 1.0 :`A` 1.0) 20.0))

(event `Delegate_HTTP_LibHv_Request`
  (params (Connection :type "HttpConnectionLhv Object Reference"))
  (`self.F_Give_Response_LibHv` Connection))

(fn `F_Give_Response_LibHv`
  (params (Connection :type "HttpConnectionLhv Object Reference"))
  (locals (LOC_Connection :type "HttpConnectionLhv Object Reference") (LOC_Querries :type String) (LOC_Client_Addr :type String) (LOC_Paths :type String) (LOC_Body :type String) (LOC_Contenty_Type :type String) (LOC_All_Headers :type String) (LOC_Single_Header :type String))
  (set `local.LOC_Connection` Connection)
  (bind (_out_value _returnvalue) (`HttpConnectionLhv.FindHeader` (`local.LOC_Connection`) "User-Agent"))
  (set `local.LOC_Single_Header` (`KismetStringLibrary.Concat_StrStr` "User-Agent = " (select `bool` _returnvalue :`true` _out_value)))
  (bind (_out_querry _out_string _returnvalue_2) (`HttpConnectionLhv.GetQuerries` (`local.LOC_Connection`)))
  (set `local.LOC_Querries` (`KismetStringLibrary.Concat_StrStr` "Querries = " (select `bool` _returnvalue_2 :`true` _out_string)))
  (bind (_out_ip _out_port _returnvalue_3) (`HttpConnectionLhv.GetClientAddress` (`local.LOC_Connection`)))
  (set `local.LOC_Client_Addr` (`KismetStringLibrary.Concat_StrStr` "Client Address = " (select `bool` _returnvalue_3 :`true` (`KismetStringLibrary.Concat_StrStr` _out_ip ":" (`KismetStringLibrary.Conv_IntToString` _out_port)))))
  (bind (_out_method _out_scheme _out_host _out_port_2 _out_path _out_url) (`HttpConnectionLhv.GetPaths` (`local.LOC_Connection`)))
  (set `local.LOC_Paths` (`KismetStringLibrary.Concat_StrStr` "Method = " _out_method " \n" "Scheme = " _out_scheme " \n" "Host = " _out_host " \n" "Port = " (`KismetStringLibrary.Conv_IntToString` _out_port_2) " \n" "Path = " _out_path " \n" "URL = " _out_url " \n" "Request Time = " (`ExtendedVarsBPLibrary.FDateTime_To_String` (`HttpConnectionLhv.RequestTime` (`local.LOC_Connection`)))))
  (bind (_out_body _out_bodysize _returnvalue_4) (`HttpConnectionLhv.GetBody` (`local.LOC_Connection`)))
  (set `local.LOC_Body` (`KismetStringLibrary.Concat_StrStr` "Body = " (select `bool` _returnvalue_4 :`true` _out_body) " \n" "Body Size = " (select `bool` _returnvalue_4 :`true` (`KismetStringLibrary.Conv_IntToString` _out_bodysize))))
  (bind (_out_content_type _out_type_string _returnvalue_5) (`HttpConnectionLhv.GetContentType` (`local.LOC_Connection`)))
  (set `local.LOC_Contenty_Type` (`KismetStringLibrary.Concat_StrStr` "Content Type = " (select `bool` _returnvalue_5 :`true` _out_type_string)))
  (bind (_out_headers _out_string_2 _returnvalue_6) (`HttpConnectionLhv.GetHeaders` (`local.LOC_Connection`)))
  (set `local.LOC_All_Headers` (`KismetStringLibrary.Concat_StrStr` "All Headers = " (select `bool` _returnvalue_6 :`true` _out_string_2)))
  (bind _returnvalue_7 (`HttpConnectionLhv.SendResponse` (`local.LOC_Connection`) (`KismetArrayLibrary.Array_Random` (`|MakeArray` "Eray" "Ezgi" "Burak")) (`|MakeMap` "Content-Type" "text/plain") "OK_200" "Text_Plain"))
  (`KismetSystemLibrary.PrintString` (`KismetStringLibrary.Concat_StrStr` "Request Sent = " (`KismetStringLibrary.Conv_BoolToString` _returnvalue_7) " \n// \n" (`local.LOC_Client_Addr`) " \n// \n" (`local.LOC_Paths`) " \n// \n" (`local.LOC_Querries`) " \n// \n" (`local.LOC_Contenty_Type`) " \n// \n" (`local.LOC_All_Headers`) " \n// \n" (`local.LOC_Body`) " \n// \n" (`local.LOC_Single_Header`)) true true (struct :`R` 1.0 :`A` 1.0) 10.0)
  (return))

(fn `UserConstructionScript`)